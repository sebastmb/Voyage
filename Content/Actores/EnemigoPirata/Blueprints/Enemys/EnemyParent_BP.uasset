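; Base pirate enemy that chases and melees the player (Mayla) with a socket-attached sword.
; PawnSensing enables AIMoveTo pursuit, while a short forward trace each tick triggers random attack montages.
; Spear overlaps during the player's SlideSpear (with brief hit cooldown) and fireballs reduce health, updating a camera-facing bar and playing hit reactions.
; Death ragdolls the mesh, disables capsule collision and pauses the sword's trace timer, before delayed destruction.
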(event OnSeePawn(PawnSensing)
  (params (Pawn :type Pawn%20Object%20Reference))
  ;[1 1 1] Event See
  (Variables|Default|SetEnemySeePlayer true))

(event OnComponentBeginOverlap(CapsuleComponent)
  (params (OverlappedComponent :type Primitive%20Component%20Object%20Reference) (OtherActor :type Actor%20Object%20Reference) (OtherComp :type Primitive%20Component%20Object%20Reference) (OtherBodyIndex :type Integer) (bFromSweep :type Boolean) (SweepResult :type Hit%20Result%20Structure%20%28by%20ref%29))
  ;[1 0.6815 0] Spear attack
  (Utilities|Casting|CastToWeapon_Spear OtherActor)
  (bind _asmayla_character_bp (Utilities|Casting|CastToMayla_CharacterBP (Game|GetPlayerCharacter 0)))
  (if (Variables|/Game/Actores/Personaje/Mayla/Mayla_CharacterBP.Mayla_CharacterBP_C|GetSlide_Spear? _asmayla_character_bp)
    (if (Variables|Default|GetCanBeHit?)
      (bind _output_get (Variables|Default|SetCurrentHealth (- (Variables|Default|GetCurrentHealth) 0.05)))
      (if (<= _output_get 0.0)
        (CallFunction|Death)
        (Utilities|FlowControl|Delay 8.0)
        (Actor|DestroyActor)
        (else
          (bind _asbarra_salud (Utilities|Casting|CastToBarraSalud (UserInterface|GetUserWidgetObject (Variables|Default|GetWidget))))
          (Progress|SetPercent (Variables|/Game/Actores/Enemy/Blueprints/BarraSalud.BarraSalud_C|GetProgressBar_54 _asbarra_salud) (Variables|Default|GetCurrentHealth))
          (Utilities|FlowControl|Sequence
            (:then_0
              (Variables|Default|SetPlayingAnimation true)
              (bind _returnvalue (Animation|PlayAnimMontage "/Game/Actores/EnemigoPirata/Animations/EnemyDamageReactMontage.EnemyDamageReactMontage" 1.0 "None"))
              (Utilities|FlowControl|Delay _returnvalue)
              (Variables|Default|SetPlayingAnimation false))
            (:then_1
              (Variables|Default|SetCanBeHit? false)
              (Utilities|FlowControl|Delay 0.32)
              (Variables|Default|SetCanBeHit? true))))))))

(event Custom|Attack
  ;[1 1 1] Event Attack
  (if (and (not (Variables|Default|GetEnemyDeath)) (Variables|Default|GetCanAttack?))
    (Variables|Default|SetCanAttack? false)
    (bind _returnvalue (Animation|PlayAnimMontage (Utilities|Array|Get(acopy) (Variables|Default|GetAttacks) (Math|Random|RandomInteger 7)) 1.0 "None"))
    (Utilities|FlowControl|Delay _returnvalue)
    (Variables|Default|SetCanAttack? true)))

(event Custom|AddWeapon
  ;[1 1 1] Add Enemy Weapon
  (bind _returnvalue (Game|SpawnActorfromClass "/Game/Actores/EnemigoPirata/Blueprints/Enemys/EnemySword_BP.EnemySword_BP_C" (Math|Transform|MakeTransform "0, 0, 0") "Undefined" 0 0))
  (bind _output_get (Variables|Default|SetEnemySwordRef _returnvalue))
  (Transformation|AttachComponentToComponent _output_get (Variables|Character|GetMesh) "ForEquipSwordw" "SnapToTarget" "SnapToTarget" "KeepRelative" true))

(event Custom|MoveToPlayer
  ;[1 1 1] MoveToPlayer
  (if (Variables|Default|GetEnemySeePlayer)
    (if (and (Variables|Default|GetCanAttack?) (not (Variables|Default|GetPlayingAnimation)))
      (AI|AIMoveTo self "0, 0, 0" (Game|GetPlayerCharacter 0) 5.0 false))))

(event EventBeginPlay
  ;[1 1 1] Events
  (Utilities|FlowControl|Sequence
    (:then_0
      (CallFunction|UpdateHealth))
    (:then_1
      (CallFunction|AddWeapon))
    (:then_2
      ;[0 1 0.07882] Health
      (bind _asbarra_salud (Utilities|Casting|CastToBarraSalud (UserInterface|GetUserWidgetObject (Variables|Default|GetWidget))))
      (Progress|SetPercent (Variables|/Game/Actores/Enemy/Blueprints/BarraSalud.BarraSalud_C|GetProgressBar_54 _asbarra_salud) (Variables|Default|GetCurrentHealth)))))

(event Collision|EventActorBeginOverlap
  (params (OtherActor :type Actor%20Object%20Reference))
  ;[1 0.008603 0] Fireball damage
  (bind _asbp_fireball (Utilities|Casting|CastToBp_Fireball OtherActor))
  (Effects|SpawnEmitteratLocation 0 (Transformation|GetActorLocation _asbp_fireball))
  (Variables|Default|SetCurrentHealth (- (Variables|Default|GetCurrentHealth) 0.25))
  (if (<= (Variables|Default|GetCurrentHealth) 0.0)
    (Actor|DestroyActor _asbp_fireball)
    (Rendering|SetVisibility (Variables|Default|GetWidget) false false)
    (CallFunction|Death)
    (Utilities|FlowControl|Delay 8.0)
    (Actor|DestroyActor)
    (else
      (bind _asbarra_salud (Utilities|Casting|CastToBarraSalud (UserInterface|GetUserWidgetObject (Variables|Default|GetWidget))))
      (Progress|SetPercent (Variables|/Game/Actores/Enemy/Blueprints/BarraSalud.BarraSalud_C|GetProgressBar_54 _asbarra_salud) (Variables|Default|GetCurrentHealth))
      (Actor|DestroyActor _asbp_fireball)
      (Variables|Default|SetPlayingAnimation true)
      (bind _returnvalue (Animation|PlayAnimMontage "/Game/Actores/EnemigoPirata/Animations/EnemyDamageReactMontage.EnemyDamageReactMontage" 1.0 "None"))
      (Utilities|FlowControl|Delay _returnvalue)
      (Variables|Default|SetPlayingAnimation false))))

(event EventTick
  (params (DeltaSeconds :type Float%20%28single-precision%29))
  (bind _returnvalue (Transformation|GetActorLocation))
  ;[1 1 1] Events
  (Utilities|FlowControl|Sequence
    (:then_0
      (CallFunction|MovetoPlayer))
    (:then_1
      ;[1 1 1] enemy attacks If player in trace
      (bind (_outhit _returnvalue_2) (Collision|LineTraceForObjects _returnvalue (+ _returnvalue (* (Transformation|GetActorForwardVector) 125.0)) (Utilities|Array|MakeArray "ObjectTypeQuery3") false 0 "None"))
      (if _returnvalue_2
        (Utilities|Casting|CastToMayla_CharacterBP (.HitActor (Collision|BreakHitResult _outhit)))
        (CallFunction|Attack)))
    (:then_2
      ;[1 1 1] Barra de salud enemigo
      (Transformation|SetWorldRotation (Variables|Default|GetWidget) (Math|Rotator|MakeRotator 0.0 0.0 (.Yaw (Math|Rotator|BreakRotator (Math|Rotator|FindLookatRotation (Transformation|GetWorldLocation (Variables|Default|GetWidget)) (Transformation|GetActorLocation (Game|GetPlayerCameraManager 0)))))) false false))))

(fn ConstructionScript)

(fn UpdateHealth
  (bind _asenemy_health (Utilities|Casting|CastToEnemy_Health (UserInterface|GetUserWidgetObject (Variables|Default|GetWidget))))
  (Progress|SetPercent (Variables|/Game/Actores/EnemigoPirata/Blueprints/Enemys/Enemy_Health.Enemy_Health_C|GetHealth _asenemy_health) (/ (Variables|Default|GetCurrentHealth) (Variables|Default|GetMaxHealth)))
  (if (<= (Variables|Default|GetCurrentHealth) 0.0)
    (CallFunction|Death))
  (return))

(fn Death
  (if (<= (Variables|Default|GetCurrentHealth) 0.0)
    (Physics|SetSimulatePhysics (Variables|Character|GetMesh) true)
    (Rendering|SetVisibility (Variables|Default|GetWidget) false false)
    (Collision|SetCollisionEnabled (Variables|Collision|GetCapsuleComponent) "NoCollision")
    (Variables|Default|SetEnemyDeath true)
    (Class|KismetSystemLibrary|PauseTimer (Variables|Default|GetEnemySwordRef) "AttackTrace")
    (return)))