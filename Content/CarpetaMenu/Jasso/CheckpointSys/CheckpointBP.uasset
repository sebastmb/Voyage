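; Checkpoint actor that shows a saved-game widget while Mayla_CharacterBP overlaps its collider and updates the "Check" save slot.
; With its Load flag true, it plays a particle burst and sound, then writes the player's location and the flag, creating the SaveGameClass object if needed.
; With Load false, it instead writes false to the existing save and prints that the checkpoint is cleared.
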(event OnComponentEndOverlap(Collider)
  (params (OverlappedComponent :type Primitive%20Component%20Object%20Reference) (OtherActor :type Actor%20Object%20Reference) (OtherComp :type Primitive%20Component%20Object%20Reference) (OtherBodyIndex :type Integer))
  (Utilities|Casting|CastToMayla_CharacterBP OtherActor)
  (Widget|RemovefromParent (stale OnComponentBeginOverlap(Collider) _returnvalue)))

(event OnComponentBeginOverlap(Collider)
  (params (OverlappedComponent :type Primitive%20Component%20Object%20Reference) (OtherActor :type Actor%20Object%20Reference) (OtherComp :type Primitive%20Component%20Object%20Reference) (OtherBodyIndex :type Integer) (bFromSweep :type Boolean) (SweepResult :type Hit%20Result%20Structure%20%28by%20ref%29))
  (bind _asmayla_character_bp (Utilities|Casting|CastToMayla_CharacterBP OtherActor))
  (bind _returnvalue (UserInterface|CreateWidget "/Game/CarpetaMenu/Jasso/CheckpointSys/SavedGame1.SavedGame1_C"))
  (UserInterface|Viewport|AddtoViewport _returnvalue 0)
  (if (Variables|Default|GetLoad?)
    (Utilities|FlowControl|Sequence
      (:then_0
        (Variables|Default|SetPlayerLocation (Transformation|GetActorLocation _asmayla_character_bp))
        (Effects|SpawnEmitteratLocation "/Game/TrailPack/Particles/Magic/Hit/P_MagicHitFinisher.P_MagicHitFinisher" (Transformation|GetActorLocation))
        (Audio|PlaySound2D "/Game/Audio/Ambiente/Magic_Shimmer.Magic_Shimmer" 1.0 1.0 0.0 0 0))
      (:then_1
        (bind _returnvalue_2 (SaveGame|DoesSaveGameExist "Check"))
        (if _returnvalue_2
          (bind _returnvalue_3 (SaveGame|LoadGamefromSlot "Check"))
          (bind _assave_game_class (Utilities|Casting|CastToSaveGameClass _returnvalue_3))
          (Variables|/Game/CarpetaMenu/Jasso/CheckpointSys/SaveGameClass.SaveGameClass_C|SetPlayerLocation _assave_game_class (Variables|Default|GetPlayerLocation))
          (Variables|Default|SetLoad? true)
          (Variables|/Game/CarpetaMenu/Jasso/CheckpointSys/SaveGameClass.SaveGameClass_C|SetLoad? _assave_game_class (Variables|Default|GetLoad?))
          (SaveGame|SaveGametoSlot _assave_game_class "Check")
          (Utilities|FlowControl|Delay 1e+01)
          (else
            (bind _returnvalue_4 (SaveGame|CreateSaveGameObject "/Game/CarpetaMenu/Jasso/CheckpointSys/SaveGameClass.SaveGameClass_C"))
            (Variables|/Game/CarpetaMenu/Jasso/CheckpointSys/SaveGameClass.SaveGameClass_C|SetPlayerLocation _returnvalue_4 (Variables|Default|GetPlayerLocation))
            (Variables|Default|SetLoad? true)
            (Variables|/Game/CarpetaMenu/Jasso/CheckpointSys/SaveGameClass.SaveGameClass_C|SetLoad? _returnvalue_4 (Variables|Default|GetLoad?))
            (SaveGame|SaveGametoSlot _returnvalue_4 "Check")
            (Utilities|FlowControl|Delay 1e+01)))))
    (else
      (bind _returnvalue_5 (SaveGame|LoadGamefromSlot "Check"))
      (bind _assave_game_class_2 (Utilities|Casting|CastToSaveGameClass _returnvalue_5))
      (Variables|Default|SetLoad? false)
      (Variables|/Game/CarpetaMenu/Jasso/CheckpointSys/SaveGameClass.SaveGameClass_C|SetLoad? _assave_game_class_2 (Variables|Default|GetLoad?))
      (SaveGame|SaveGametoSlot _assave_game_class_2 "Check")
      (Development|PrintString "Checkpoint cleared" true true "(R=0.000000,G=0.489583,B=0.017477,A=1.000000)")
      (Utilities|FlowControl|Delay 1e+01))))

(event EventBeginPlay)

(event Collision|EventActorBeginOverlap
  (params (OtherActor :type Actor%20Object%20Reference)))

(event EventTick
  (params (DeltaSeconds :type Float%20%28single-precision%29)))

(fn ConstructionScript)